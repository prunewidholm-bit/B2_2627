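; Lava hazard that kills the third-person character on box overlap when IsDeadly is set.
; It hands the character to the level's Killzone_BP, calls its DEAD function, then fades the camera and shows a death message through the HUD.
; After a short delay, it teleports the Player reference to its saved checkpoint or a hard-coded start location, based on RespawnAtCheckpoint, with a matching reset message.
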(event OnComponentBeginOverlap(Box)
  (params (OverlappedComponent :type Primitive%20Component%20Object%20Reference) (OtherActor :type Actor%20Object%20Reference) (OtherComp :type Primitive%20Component%20Object%20Reference) (OtherBodyIndex :type Integer) (bFromSweep :type Boolean) (SweepResult :type Hit%20Result%20Structure%20%28by%20ref%29))
  (bind _asbp_third_person_character (Utilities|Casting|CastToBP_ThirdPersonCharacter OtherActor))
  (if (Variables|Default|GetisDeadly)
    (bind _returnvalue (Actor|GetActorOfClass "/Game/B2/00_BuildMyLevel/DONT_TOUCH/Killzone_BP.Killzone_BP_C"))
    (Variables|/Game/B2/00_BuildMyLevel/DONT_TOUCH/Killzone_BP.Killzone_BP_C|Setplayer _returnvalue _asbp_third_person_character)
    (Default|DEAD _returnvalue)
    (CameraFades|StartCameraFade :self (Game|GetPlayerCameraManager 0) :ToAlpha 1.0 :Duration 0.5)
    (Utilities|FlowControl|Delay 0.5)
    (Class|BPIInterface|Notif(Message) (HUD|GetHUD (Game|GetPlayerController 0)) "YOU DIED :(")
    (if (Variables|Components|GetrespawnAtCheckpoint)
      (Transformation|SetActorLocation (Variables|Components|Getplayer) (Variables|/Game/ThirdPerson/Blueprints/BP_ThirdPersonCharacter.BP_ThirdPersonCharacter_C|GetcheckpointLoc (Variables|Components|Getplayer)) false false)
      (Class|BPIInterface|Notif(Message) (HUD|GetHUD (Game|GetPlayerController 0)) "Reset From Last Checkpoint")
      (else
        (Transformation|SetActorLocation (Variables|Components|Getplayer) "-1210.000000,-1840.000000,10.000000" false false)
        (Class|BPIInterface|Notif(Message) (HUD|GetHUD (Game|GetPlayerController 0)) "Reset From Start")))))

(event EventBeginPlay)

(event Collision|EventActorBeginOverlap
  (params (OtherActor :type Actor%20Object%20Reference)))

(event EventTick
  (params (DeltaSeconds :type Float%20%28single-precision%29)))

(fn ConstructionScript)