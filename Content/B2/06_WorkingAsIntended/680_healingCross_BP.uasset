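; Healing cross pickup that the AsIntended character collects by overlapping its HealBox.
; On pickup it finds the 680_HealingZone actor, subtracts a fixed amount from that zone's CurrentHp rather than adding to it, calls RespawnCross on it and destroys itself.
; A timeline started on BeginPlay spins the cross by a fixed yaw step per update, so rotation speed depends on frame rate.
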(event OnComponentBeginOverlap(HealBox)
  (params (OverlappedComponent :type Primitive%20Component%20Object%20Reference) (OtherActor :type Actor%20Object%20Reference) (OtherComp :type Primitive%20Component%20Object%20Reference) (OtherBodyIndex :type Integer) (bFromSweep :type Boolean) (SweepResult :type Hit%20Result%20Structure%20%28by%20ref%29))
  (Utilities|Casting|CastToBP_AsIntendedCharacter OtherActor)
  (bind _returnvalue (Actor|GetActorOfClass "/Game/B2/06_WorkingAsIntended/680_HealingZone.680_HealingZone_C"))
  (Variables|/Game/B2/06_WorkingAsIntended/680_HealingZone.680_HealingZone_C|SetCurrentHp _returnvalue (- (Variables|/Game/B2/06_WorkingAsIntended/680_HealingZone.680_HealingZone_C|GetCurrentHp _returnvalue) 1e+01))
  (Default|RespawnCross _returnvalue)
  (Actor|DestroyActor))

(fn ConstructionScript)

(event EventBeginPlay
  (Timeline|TL_Rotate PlayFromStart
    (:Update
      (Class|SceneComponent|AddWorldTransform (Variables|Default|GetDefaultSceneRoot) (Math|Transform|MakeTransform "0, 0, 0" "0.000000,2.000000,0.000000" "1.000000,1.000000,1.000000") false false))))